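; Base player character Blueprint that sets up default locomotion and provides debug controls for switching animation layers.
; On BeginPlay it runs the parent logic, sets the movement type to strafe-desired and calls DebugTurnInPlace with false.
; Three debug keys set the AnimComponent's layer tag to switch between unarmed and weapon animation layers.
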(event EventBeginPlay
  (|CallParentFunction)
  (Class|TurninPlaceStatics|SetCharacterMovementType 0 "StrafeDesired")
  (Class|TurninPlaceStatics|DebugTurninPlace false))

(event Collision|EventActorBeginOverlap
  (params (OtherActor :type Actor%20Object%20Reference)))

(event Input|KeyboardEvents|DebugKey1
  (params (Key :type Key%20Structure :default "None") (ActionValue :type Input%20Action%20Value%20Structure))
  (:Pressed
    (Class|AnimComponent|SetAnimLayerTag (Variables|Default|GetAnimComponent) "Unarmed")))

(event Input|KeyboardEvents|DebugKey2
  (params (Key :type Key%20Structure :default "None") (ActionValue :type Input%20Action%20Value%20Structure))
  (:Pressed
    (Class|AnimComponent|SetAnimLayerTag (Variables|Default|GetAnimComponent) "Pistol")))

(event Input|KeyboardEvents|DebugKey3
  (params (Key :type Key%20Structure :default "None") (ActionValue :type Input%20Action%20Value%20Structure))
  (:Pressed
    (Class|AnimComponent|SetAnimLayerTag (Variables|Default|GetAnimComponent) "Rifle")))

(fn ConstructionScript)